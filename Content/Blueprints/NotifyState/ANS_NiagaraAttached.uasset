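; Animation notify state that spawns a Niagara effect on the mesh owner for the duration of the notify window.
; Begin adds and tags a Niagara component with the notify's display name, then attaches and activates it on an owner component matching a configured class and tag.
; End finds it by that tag, deactivates it, and destroys it immediately or hands delayed destruction to BP_BaseCharacter when a delay is set.
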(fn ReceivedNotifyBegin
  (params (MeshComp :type Skeletal%20Mesh%20Component%20Object%20Reference) (Animation :type Anim%20Sequence%20Base%20Object%20Reference) (TotalDuration :type Float%20%28single-precision%29) (EventReference :type Anim%20Notify%20Event%20Reference%20Structure%20%28by%20ref%29))
  (bind _returnvalue (Game|AddComponentbyClass (Components|GetOwner MeshComp) 0 "/Script/Niagara.NiagaraComponent"))
  (bind _output_get (LocalVariables|SetNiagaraComponent _returnvalue))
  (Class|NiagaraComponent|SetAsset _output_get (Variables|Default|GetNiagaraSystem) true)
  (Utilities|Array|Add (Variables|/Script/Engine.ActorComponent|GetComponentTags (LocalVariables|GetNiagaraComponent)) (Utilities|String|StringToName (Utilities|GetDisplayName self)))
  (for _array_element (Actor|GetComponentsByClass (Components|GetOwner MeshComp) (Variables|Default|GetAttachToComponentClass))
    (if (Components|ComponentHasTag _array_element (Variables|Default|GetAttachToComponentTag))
      (LocalVariables|SetComponentToAttach _array_element)))
  (if (Utilities|IsValid (LocalVariables|GetComponentToAttach))
    (Transformation|AttachComponentToComponent (LocalVariables|GetNiagaraComponent) (.AsScene%20Component (Utilities|Casting|CastToSceneComponent (LocalVariables|GetComponentToAttach))) "None" "KeepRelative" "KeepRelative" "KeepRelative" true)
    (Components|Activation|Activate (LocalVariables|GetNiagaraComponent) true)
    (return true)
    (else
      (return false))))

(fn ReceivedNotifyEnd
  (params (MeshComp :type Skeletal%20Mesh%20Component%20Object%20Reference) (Animation :type Anim%20Sequence%20Base%20Object%20Reference) (EventReference :type Anim%20Notify%20Event%20Reference%20Structure%20%28by%20ref%29))
  (bind _returnvalue (Components|GetOwner MeshComp))
  (bind (_asbp_base_character _bsuccess) (Utilities|Casting|CastToBP_BaseCharacter _returnvalue))
  (for _array_element (Actor|GetComponentsByClass (Components|GetOwner MeshComp) "/Script/Niagara.NiagaraComponent")
    (if (Components|ComponentHasTag _array_element (Utilities|String|StringToName (Utilities|GetDisplayName self)))
      (LocalVariables|SetNiagaraComponent _array_element)))
  (if (Utilities|IsValid (LocalVariables|GetNiagaraComponent))
    (Components|Activation|Deactivate (LocalVariables|GetNiagaraComponent))
    (if (and (> (Variables|Default|GetTimeToDestroy) 0.0) _bsuccess)
      (Default|DestroyNiagaraComponent _asbp_base_character (Variables|Default|GetTimeToDestroy) (LocalVariables|GetNiagaraComponent))
      (return true)
      (else
        (Components|DestroyComponent (LocalVariables|GetNiagaraComponent))
        (return true)))
    (else
      (return false))))