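; Anim notify state that gives a melee attack its launch hit on enemies during the active window of the animation.
; Each tick it sphere-traces on the Visibility channel between the mesh's CollisionStart and CollisionEnd sockets and casts the hit actor to BP_BaseEnemyCharacter.
; A HitEnemies list, cleared on begin, stops repeat hits; each new enemy gets MeleeHitLaunch and triggers a launch camera shake at player 0's controller.
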(fn ReceivedNotifyTick
  (params (MeshComp :type Skeletal%20Mesh%20Component%20Object%20Reference) (Animation :type Anim%20Sequence%20Base%20Object%20Reference) (FrameDeltaTime :type Float%20%28single-precision%29) (EventReference :type Anim%20Notify%20Event%20Reference%20Structure%20%28by%20ref%29))
  (bind _returnvalue (Game|GetPlayerController MeshComp))
  (bind (_outhit _returnvalue_2) (Collision|SphereTraceByChannel MeshComp (Transformation|GetSocketLocation MeshComp "CollisionStart") (Transformation|GetSocketLocation MeshComp "CollisionEnd") 2e+01 "TraceTypeQuery1" false 0 "None"))
  (if _returnvalue_2
    (bind _asbp_base_enemy_character (Utilities|Casting|CastToBP_BaseEnemyCharacter (.HitActor (Collision|BreakHitResult _outhit))))
    (if (not (Utilities|Array|ContainsItem (Variables|Default|GetHitEnemies) _asbp_base_enemy_character))
      (Utilities|Array|Add (Variables|Default|GetHitEnemies) _asbp_base_enemy_character)
      (Default|MeleeHitLaunch _asbp_base_enemy_character)
      (Camera|PlayWorldCameraShake _returnvalue "/Game/Blueprints/CameraShake/BP_CSLaunchCharacter.BP_CSLaunchCharacter_C" (Transformation|GetActorLocation _returnvalue) 5e+02 8e+02)
      (return false))))

(fn ReceivedNotifyBegin
  (params (MeshComp :type Skeletal%20Mesh%20Component%20Object%20Reference) (Animation :type Anim%20Sequence%20Base%20Object%20Reference) (TotalDuration :type Float%20%28single-precision%29) (EventReference :type Anim%20Notify%20Event%20Reference%20Structure%20%28by%20ref%29))
  (Utilities|Array|Clear (Variables|Default|GetHitEnemies))
  (return false))