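; Anim notify state that runs the hero's melee hit detection during an attack montage window.
; Each tick it sphere-traces between the weapon's collision sockets, extended sideways by TraceLength.
; Each enemy hit first in that window takes the current montage's damage, triggers a world shake and adds a combo.
; Any pawn hit also shakes the player camera on every tick; the hit list clears on begin.
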(fn ReceivedNotifyTick
  (params (MeshComp :type Skeletal%20Mesh%20Component%20Object%20Reference) (Animation :type Anim%20Sequence%20Base%20Object%20Reference) (FrameDeltaTime :type Float%20%28single-precision%29) (EventReference :type Anim%20Notify%20Event%20Reference%20Structure%20%28by%20ref%29))
  (bind _returnvalue (Components|GetOwner MeshComp))
  (bind _returnvalue_2 (Game|GetPlayerController MeshComp))
  (bind _asbp_hero (Utilities|Casting|CastToBP_Hero _returnvalue))
  (bind (_outhit _returnvalue_3) (Collision|SphereTraceByChannel MeshComp (Transformation|GetSocketLocation MeshComp "CollisionStart") (+ (Transformation|GetSocketLocation MeshComp "CollisionEnd") (* (Math|Vector|GetRightVector (Transformation|GetSocketRotation MeshComp "CollisionEnd")) (Variables|Default|GetTraceLength))) 2e+01 "TraceTypeQuery1" false 0 "None"))
  (if _returnvalue_3
    (Utilities|FlowControl|Sequence
      (:then_0
        (bind _asbp_base_enemy_character (Utilities|Casting|CastToBP_BaseEnemyCharacter (.HitActor (Collision|BreakHitResult _outhit))))
        (if (not (Utilities|Array|ContainsItem (Variables|Default|GetEnemyHit) _asbp_base_enemy_character))
          (Utilities|Array|Add (Variables|Default|GetEnemyHit) _asbp_base_enemy_character)
          (Game|Damage|ApplyDamage (.HitActor (Collision|BreakHitResult _outhit)) (.damage (Variables|/Game/Blueprints/Character/BP_Hero.BP_Hero_C|GetCurrentAttackMontageDetail _asbp_hero)) _returnvalue_2 _returnvalue_2 "/Script/Engine.DamageType")
          (Camera|PlayWorldCameraShake _returnvalue_2 "/Game/Blueprints/CameraShake/BP_CSLightAttack.BP_CSLightAttack_C" (.Location (Collision|BreakHitResult _outhit)) 5e+02 1e+03)
          (Default|AddCombo (Variables|/Game/Blueprints/Character/BP_Hero.BP_Hero_C|GetBPC_ComboCounter _asbp_hero))
          (return false)))
      (:then_1
        (Utilities|Casting|CastToPawn (.HitActor (Collision|BreakHitResult _outhit)))
        (CameraShakes|StartCameraShake (Game|GetPlayerCameraManager MeshComp) "/Game/Developers/sherwynr/CameraSkakh/BP_CameraShaike.BP_CameraShaike_C" (Variables|Default|GetScale) "CameraLocal" "0, 0, 0")))))

(fn ReceivedNotifyBegin
  (params (MeshComp :type Skeletal%20Mesh%20Component%20Object%20Reference) (Animation :type Anim%20Sequence%20Base%20Object%20Reference) (TotalDuration :type Float%20%28single-precision%29) (EventReference :type Anim%20Notify%20Event%20Reference%20Structure%20%28by%20ref%29))
  (Utilities|Array|Clear (Variables|Default|GetEnemyHit))
  (return false))