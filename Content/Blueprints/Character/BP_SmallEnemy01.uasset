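; Small enemy character that reacts to damage with a hit flash, electric VFX, directional montages and knockback away from the player.
; Dot products against the player direction pick montages from a DataTable row, with high damage selecting heavy variants, stronger knockback and a fallen state.
; Melee launches and airborne hits feed a downfall loop, with get-up montages on landing.
; Hit and recovery states are reported to the BP_AIC_Base AI controller.
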(event Custom|PlayLaunchMontage
  (Animation|Montage|PlayMontage (Variables|Character|GetMesh) "/Game/ExternalAssets/GhostSamurai_Bundle/GhostSamurai/Katana/Apose/Hit/Inplace/GhostSamurai_APose_Hit_Up_Inplace_Montage.GhostSamurai_APose_Hit_Up_Inplace_Montage"
    (:OnBlendOut
      (CallFunction|DownfallLoop))))

(event Custom|DownfallLoop
  (Animation|Montage|PlayMontage (Variables|Character|GetMesh) "/Game/ExternalAssets/GhostSamurai_Bundle/GhostSamurai/Katana/Apose/Hit/Inplace/GhostSamurai_APose_Air__DownLoop_Inplace_Montage.GhostSamurai_APose_Air__DownLoop_Inplace_Montage"
    (:then
      (Variables|Default|SetbDownFall true))))

(event Custom|HitFlash
  (Variables|Default|SetExisting%20Mats (Rendering|Material|GetMaterials (Variables|Character|GetMesh)))
  (Rendering|Material|SetMaterial (Variables|Character|GetMesh) 0 "/Game/Character/Material/HitMat/M_Enemy_Hit.M_Enemy_Hit")
  (Rendering|Material|SetMaterial (Variables|Character|GetMesh) 1 "/Game/Character/Material/HitMat/M_Enemy_Hit.M_Enemy_Hit")
  (Utilities|FlowControl|Delay 0.09)
  (Rendering|Material|SetMaterial (Variables|Character|GetMesh) 0 "/Game/Character/MaterialInstances/SmallEnemy01/M_SmallEnemy01_Body.M_SmallEnemy01_Body")
  (Rendering|Material|SetMaterial (Variables|Character|GetMesh) 1 "/Game/Character/MaterialInstances/SmallEnemy01/M_SmallEnemy01_ChestLogo.M_SmallEnemy01_ChestLogo"))

(event Custom|HitVFX
  (Effects|SpawnEmitteratLocation "/Game/Realistic_Starter_VFX_Pack_Vol2/Particles/Destruction/P_Destruction_Electric.P_Destruction_Electric" (Transformation|GetActorLocation) "0, 0, 0" "0.050000,0.050000,0.050000")
  (Effects|SpawnEmitteratLocation "/Game/Realistic_Starter_VFX_Pack_Vol2/Particles/Destruction/P_Destruction_Electric.P_Destruction_Electric" (Transformation|GetActorLocation) "0, 0, 0" "0.050000,0.050000,0.050000"))

(event Custom|GetUp
  (if (Variables|Default|GetbDownFall)
    (Variables|Default|SetbDownFall false)
    (Animation|Montage|PlayMontage (Variables|Character|GetMesh) "/Game/ExternalAssets/GhostSamurai_Bundle/GhostSamurai/Katana/Apose/Hit/Inplace/GhostSamurai_APose_Hit_Up_FallDown_Inplace_Montage.GhostSamurai_APose_Hit_Up_FallDown_Inplace_Montage"
      (:OnBlendOut
        (Animation|Montage|PlayMontage (Variables|Character|GetMesh) "/Game/ExternalAssets/GhostSamurai_Bundle/GhostSamurai/Katana/Apose/Hit/Inplace/GhostSamurai_APose_Hit_Up_GetUP_Inplace_Montage.GhostSamurai_APose_Hit_Up_GetUP_Inplace_Montage"
          (:then
            (Default|GotHit (.AsBP%20AIC%20Base (Utilities|Casting|CastToBP_AIC_Base (AI|GetAIController self))) false false)))))))

(event Custom|playAiAnimation
  (Animation|Montage|PlayMontage (Variables|Character|GetMesh) "/Game/ExternalAssets/GhostSamurai_Bundle/GhostSamurai/Katana/Apose/Attack/Root/GhostSamurai_APose_Attack02_4_Root_Montage.GhostSamurai_APose_Attack02_4_Root_Montage"
    (:then
      (Development|PrintString "Hello"))))

(event Game|Damage|EventAnyDamage
  (params (Damage :type Float%20%28single-precision%29) (DamageType :type Damage%20Type%20Object%20Reference) (InstigatedBy :type Controller%20Object%20Reference) (DamageCauser :type Actor%20Object%20Reference))
  (Utilities|FlowControl|Sequence
    (:then_0
      (CallFunction|HitFlash)
      (CallFunction|HitVFX))
    (:then_1
      (CallFunction|SetinAirCondition))
    (:then_2
      (Default|GotHit (.AsBP%20AIC%20Base (Utilities|Casting|CastToBP_AIC_Base (AI|GetAIController self))) (Variables|Default|GetbIsinAir) false))
    (:then_3
      (CallFunction|SetHitMontage Damage))
    (:then_4
      (Animation|Montage|PlayMontage (Variables|Character|GetMesh) (Variables|Default|GetHitMontage%20to%20Play)
        (:then
          (Character|LaunchCharacter (* (|GetDirection) (Variables|Default|GetLaunchVelocity)) true true))
        (:OnCompleted
          (if (Variables|Default|GetbIsinAir)
            (CallFunction|DownfallLoop)
            (elif (Variables|Default|GetbDownFall)
              (CallFunction|GetUp))))))))

(event EventBeginPlay
  (bind _returnvalue (Utilities|GetDataTableRow "/Game/Data/DataTable/DT_HitreactionMontages.DT_HitreactionMontages" "SmallEnemy")
    (:then
      (Variables|Default|SetHitReaction _returnvalue))))

(event EventOnLanded
  (params (Hit :type Hit%20Result%20Structure%20%28by%20ref%29))
  (CallFunction|GetUp))

(fn ConstructionScript)

(fn SetHitMontage
  (params (AppliedDamge :type Float%20%28double-precision%29))
  (bind _returnvalue (Transformation|GetActorForwardVector))
  (bind _returnvalue_2 (|GetDirection_2))
  (bind _hitreaction (Variables|Default|GetHitReaction))
  (bind _hitreaction_2 (Variables|Default|GetHitReaction))
  (bind _hitreaction_3 (Variables|Default|GetHitReaction))
  (bind _hitreaction_4 (Variables|Default|GetHitReaction))
  (bind _returnvalue_3 (Math|Vector|DotProduct _returnvalue_2 _returnvalue))
  (if (Variables|Default|GetbIsinAir)
    (Variables|Default|SetHitMontage%20to%20Play "/Game/ExternalAssets/GhostSamurai_Bundle/GhostSamurai/Katana/Apose/Hit/Inplace/InAirHit.InAirHit")
    (elif (> _returnvalue_3 0.5)
      (Utilities|NewMacro (.hitreactionfront (.heavy _hitreaction_3)) (.hitreactionfront (.light _hitreaction_3)))
      (elif (< _returnvalue_3 -0.5)
        (Utilities|NewMacro (.OutItem (Utilities|Array|Random (.hitreactionback (.heavy _hitreaction)))) (.OutItem (Utilities|Array|Random (.hitreactionback (.light _hitreaction)))))
        (elif (>= (Math|Vector|DotProduct (|GetDirection_2_2) (Transformation|GetActorRightVector)) 0.5)
          (Utilities|NewMacro (.hitreactionleft (.heavy _hitreaction_4)) (.hitreactionleft (.light _hitreaction_4)))
          (else
            (Utilities|NewMacro (.hitreactionright (.heavy _hitreaction_2)) (.hitreactionright (.light _hitreaction_2)))))))))

(fn MeleeHitLaunch
  (|CallParentFunction)
  (Character|Jump)
  (CallFunction|PlayLaunchMontage))

(fn SetinAirCondition
  (bind _output_get (Variables|Default|SetbIsinAir (or (AI|Components|NavMovement|IsFalling (Variables|Character|GetCharacterMovement)) (Utilities|Enum|Equal(Enum) (Variables|/Script/Engine.CharacterMovementComponent|GetMovementMode (Variables|Character|GetCharacterMovement)) "MOVE_Flying"))))
  (if _output_get
    (Variables|Default|SetLaunchVelocity 0.0)
    (else
      (Variables|Default|SetLaunchVelocity 1.2e+03))))