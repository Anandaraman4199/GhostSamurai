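; Actor component that picks the nearest enemy to its owner as the current target.
; On BeginPlay it adds a sphere collision to the owner, sized by a targeting radius.
; Each tick it measures 2D distance to overlapping BP_BaseEnemyCharacter actors and stores the closest as TargetingEnemy, or None when none overlap.
; An optional debug mode draws spheres on candidates and the chosen target.
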(event EventBeginPlay
  (bind _returnvalue (Game|AddComponentbyClass (Components|GetOwner) "/Script/Engine.SphereComponent" false))
  (Variables|Default|SetSphereCollision _returnvalue)
  (Components|Sphere|SetSphereRadius (Variables|Default|GetSphereCollision) (Variables|Default|GetTargetingSystemRadius) true))

(event EventTick
  (params (DeltaSeconds :type Float%20%28single-precision%29))
  (bind _distances (Variables|Default|GetDistances))
  (bind _indexofminvalue (Math|Float|MinOfFloatArray _distances))
  (Variables|Default|SetOverlapping%20Actors (Collision|GetOverlappingActors (Variables|Default|GetSphereCollision) "/Game/_Core/Blueprints/Character/BP_BaseEnemyCharacter.BP_BaseEnemyCharacter_C" :!class /Script/Engine.PrimitiveComponent))
  (for _array_element (Variables|Default|GetOverlapping%20Actors)
    (Utilities|Array|Add (Variables|Default|GetDistances) (Math|Vector|Distance2D(Vector) (Transformation|GetActorLocation (Components|GetOwner)) (Transformation|GetActorLocation _array_element)))
    (if (Variables|Default|GetDebug)
      (CallFunction|DebugLocationwithSphere (Transformation|GetActorLocation _array_element) (Utilities|GetDisplayName _array_element) 5e+01 "(R=0.000000,G=0.089617,B=1.000000,A=1.000000)")))
  (if (>= _indexofminvalue 0)
    (Utilities|FlowControl|Sequence
      (:then_0
        (Variables|Default|SetTargetingEnemy (Utilities|Array|Get(acopy) (Variables|Default|GetOverlapping%20Actors) _indexofminvalue)))
      (:then_1
        (if (Variables|Default|GetDebug)
          (CallFunction|DebugLocationwithSphere (Transformation|GetActorLocation (Variables|Default|GetTargetingEnemy)) "" 3e+01 "(R=0.171052,G=1.000000,B=0.000000,A=1.000000)")))
      (:then_2
        (Utilities|Array|Clear (Variables|Default|GetDistances))))
    (else
      (Variables|Default|SetTargetingEnemy 0))))