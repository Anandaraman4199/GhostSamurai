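; BPC_ComboCounter is a component that counts combo hits and shows the count on screen.
; It creates a WBP_ComboCount widget on BeginPlay and adds it to the viewport.
; AddCombo increments the count, restarts a reset timer, marks the combo active and updates the widget.
; When the timer expires, ResetCombos zeroes the count, clears the active flag and refreshes the widget.
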(event Custom|AddCombo
  (Math|Integer|IncrementInt (Variables|Default|GetComboCount)
    (:%20%20
      (Utilities|Time|ClearandInvalidateTimerbyHandle (Variables|Default|GetComboTimerHandle))
      (Utilities|Time|SetTimerbyFunctionName 0 "ResetCombos" (Variables|Default|GetComboResetTime))
      (Variables|Default|SetbIsComboActive true)
      (Default|UpdateComboCount (Variables|Default|GetWBP_ComboCount) (Variables|Default|GetComboCount)))))

(event EventBeginPlay
  (bind _returnvalue (UserInterface|CreateWidget "/Game/Blueprints/UI/WBP_ComboCount.WBP_ComboCount_C"))
  (bind _output_get (Variables|Default|SetWBP_ComboCount _returnvalue))
  (UserInterface|Viewport|AddtoViewport _output_get 0))

(event EventTick
  (params (DeltaSeconds :type Float%20%28single-precision%29)))

(fn ResetCombos
  (Variables|Default|SetComboCount 0)
  (Variables|Default|SetbIsComboActive false)
  (Default|UpdateComboCount (Variables|Default|GetWBP_ComboCount) (Variables|Default|GetComboCount)))