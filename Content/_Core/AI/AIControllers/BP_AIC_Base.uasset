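; Base AI controller that starts a behavior tree on BeginPlay and handles hit reactions for its controlled pawn.
; GotHit sets a flag, which a retriggerable delay clears after a short window for grounded hits.
; Airborne hits instead switch the pawn's movement to Flying briefly, then to Walking, leaving the flag set.
; Retriggerable delays let repeated hits extend either window.
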(event Custom|GotHit
  (params (bIsInAir :type Boolean))
  (Variables|Default|SetbGotHit true)
  (if bIsInAir
    (Pawn|Components|CharacterMovement|SetMovementMode (Actor|GetComponentbyClass (Pawn|GetControlledPawn) "/Script/Engine.CharacterMovementComponent") "MOVE_Flying" 0)
    (Utilities|FlowControl|RetriggerableDelay 0.35)
    (Pawn|Components|CharacterMovement|SetMovementMode (Actor|GetComponentbyClass (Pawn|GetControlledPawn) "/Script/Engine.CharacterMovementComponent") "MOVE_Walking" 0)
    (else
      (Utilities|FlowControl|RetriggerableDelay 2.0)
      (Variables|Default|SetbGotHit false))))

(event EventBeginPlay
  (AI|RunBehaviorTree (Variables|Initialization|GetBehaviorTree)))

(fn ConstructionScript)