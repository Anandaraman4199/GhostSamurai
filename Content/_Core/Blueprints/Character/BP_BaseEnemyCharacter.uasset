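; Base enemy character Blueprint that configures itself from a data table row when play begins.
; BeginPlay looks up the row set in its initialization row handle and sets max walk speed from it, with a small random offset so enemies vary in pace.
; A missing row prints an on-screen error naming the class.
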(event EventBeginPlay
  (CallFunction|InitializefromDataTable))

(event Collision|EventActorBeginOverlap
  (params (OtherActor :type Actor%20Object%20Reference)))

(event EventTick
  (params (DeltaSeconds :type Float%20%28single-precision%29)))

(fn ConstructionScript
  (|CallParentFunction))

(fn InitializefromDataTable
  (bind _initialization_data_table_row (Variables|Initialization|GetInitialization%20Data%20Table%20Row))
  (bind _returnvalue (Utilities|GetDataTableRow (.datatable _initialization_data_table_row) (.rowname _initialization_data_table_row))
    (:then
      (Variables|/Script/Engine.CharacterMovementComponent|SetMaxWalkSpeed (Variables|Character|GetCharacterMovement) (+ (Math|Random|RandomFloatinRange -5e+01 5e+01) (Utilities|Struct|BreakF_Enemy_Initialization _returnvalue))))
    (:RowNotFound
      (Development|PrintString (Utilities|String|Append (Utilities|GetClassDisplayName (Utilities|GetClass self)) " : Initialization Data Table Row is not found.") true true "(R=1.000000,G=0.020756,B=0.000000,A=1.000000)" 1e+01 "RowNotFound"))))